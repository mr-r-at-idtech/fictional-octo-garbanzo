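; Default player controller that handles first-level movement and look input for the player's Default_Character.
; On BeginPlay it caches the game instance and the player character through casts.
; Movement axes push the character along forward and right vectors from a yaw-only control rotation, computed by the GetRot helper, so camera pitch does not affect movement direction.
; Look axes feed pitch and yaw input directly to the controller.
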(event `self.ReceiveBeginPlay`
  (`|ExecutionSequence`
    (:`then_0`
      (`self.InitializeGameInstance`))
    (:`then_1`
      (`self.InitializePlayerCharacter`))))

(event `InputAxis|MoveForward/Back`
  (params (AxisValue :type "Float (single-precision)"))
  (bind (_forward _right _as_default_character) (`self.GetRot`))
  (`Pawn.AddMovementInput` _as_default_character _forward AxisValue false))

(event `InputAxis|MoveLeft/Right`
  (params (AxisValue :type "Float (single-precision)"))
  (bind (_forward _right _as_default_character) (`self.GetRot`))
  (`Pawn.AddMovementInput` _as_default_character _right AxisValue false))

(event `InputAxis|LookUp/Down`
  (params (AxisValue :type "Float (single-precision)"))
  (`self.AddPitchInput` AxisValue))

(event `InputAxis|LookLeft/Right`
  (params (AxisValue :type "Float (single-precision)"))
  (`self.AddYawInput` AxisValue))

(fn `GetRot`
  (returns (Forward :type "Vector Structure") (Right :type "Vector Structure") (`As Default Character` :type "/Game/Blueprints/Player/Default_Character Object Reference"))
  (bind _as_default_character (`self.As Default Character`))
  (bind (_returnvalue_roll _returnvalue_pitch _returnvalue_yaw) (`KismetMathLibrary.BreakRotator` (`Pawn.GetControlRotation` _as_default_character)))
  (bind _returnvalue (`KismetMathLibrary.MakeRotator` 0.0 0.0 _returnvalue_yaw))
  (return (`KismetMathLibrary.GetForwardVector` _returnvalue) (`KismetMathLibrary.GetRightVector` _returnvalue) _as_default_character))

(fn `InitializeGameInstance`
  (set `self.GameInstance` (cast `/Game/Blueprints/GameMode/Default_GameInstance` (`GameplayStatics.GetGameInstance`) :!pure true)))

(fn `InitializePlayerCharacter`
  (set `self.As Default Character` (cast `/Game/Blueprints/Player/Default_Character` (`GameplayStatics.GetPlayerCharacter` 0) :!pure true)))

(fn `UserConstructionScript`)