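; Player character Blueprint that runs a two-slot gun system with scoping, switching, ammo and reloading.
; BeginPlay builds per-weapon arrays for AR, Pistol and Tactical Rifle, then a 0.01-second Delay loop refreshes the active model, attachment points, cube hands and ammo.
; Attack spawns projectiles in automatic, single or three-round burst mode.
; Reload, aiming and recoil are animated procedurally with MoveComponentTo, though burst fire skips the recoil macro.
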(event `InputAction|Reload`
  (params (Key :type "Key Structure"))
  (bind _childactor (`self.ChildActor`))
  (bind _cube (`self.Cube`))
  (bind _maxammoarray (`self.MaxAmmoArray`))
  (bind _output (`|GetArrayItem` (`self.Reload Type Array`) (`self.CurrentWeapon`)))
  (bind _relativelocation (`SceneComponent.RelativeLocation` (`self.bolt`)))
  (bind _relativelocation_2 (`SceneComponent.RelativeLocation` (`self.Mag`)))
  (:`Pressed`
    (set `self.Not Reloading` false)
    (if (== _output 2)
      (`KismetSystemLibrary.MoveComponentTo` _childactor (80.0 37.0 13.0) (struct :`Pitch` 45.0))
      (elif (== _output 3)
        (`KismetSystemLibrary.MoveComponentTo` _childactor (70.0 37.0 -13.0) (struct :`Roll` 45.0))
        (else
          (`KismetSystemLibrary.MoveComponentTo` _childactor (80.0 37.0 -13.0)))))
    (`KismetSystemLibrary.MoveComponentTo` _cube _relativelocation_2 (struct :`Yaw` 45.0))
    (`GameplayStatics.PlaySoundAtLocation` "/Game/StarterContent/Audio/Record-_online-voice-recorder_com_.Record-_online-voice-recorder_com_" _relativelocation_2 (struct) 1.0 1.0 0.0 null null null)
    (`KismetSystemLibrary.MoveComponentTo` _cube (`KismetMathLibrary.MakeVector` (.x _relativelocation_2) (.y _relativelocation_2) (- (.z _relativelocation_2) 180.0)) (struct :`Yaw` 45.0) false false 0.4)
    (`KismetSystemLibrary.MoveComponentTo` _cube _relativelocation_2 (struct :`Yaw` 45.0) false false 0.4)
    (`GameplayStatics.PlaySoundAtLocation` "/Game/StarterContent/Audio/Record-_online-voice-recorder_com_.Record-_online-voice-recorder_com_" (0.0 0.0 0.0) (struct) 1.0 1.0 0.0 null null null)
    (`KismetSystemLibrary.MoveComponentTo` _cube _relativelocation (struct :`Yaw` 45.0))
    (`KismetSystemLibrary.MoveComponentTo` _cube (`KismetMathLibrary.MakeVector` (- (.x _relativelocation) 20.0) (.y _relativelocation) (.z _relativelocation)) (struct :`Yaw` 45.0) false false 0.1)
    (`GameplayStatics.PlaySoundAtLocation` "/Game/StarterContent/Audio/Record-_online-voice-recorder_com_.Record-_online-voice-recorder_com_" (0.0 0.0 0.0) (struct) 1.0 1.0 0.0 null null null)
    (if (== (`self.WhichWeapon`) 0)
      (set `self.PrimaryAmmo` (`|GetArrayItem` _maxammoarray (`self.Primary`)))
      (else
        (set `self.SecondaryAmmo` (`|GetArrayItem` _maxammoarray (`self.Secondary`)))))
    (`|ExecutionSequence`
      (:`then_0`
        (`KismetSystemLibrary.MoveComponentTo` _childactor (62.0 37.0 -13.0))
        (set `self.Not Reloading` true))
      (:`then_1`
        (`KismetSystemLibrary.MoveComponentTo` _cube (`SceneComponent.RelativeLocation` (`self.Grip`)) (struct :`Yaw` 45.0))))))

(event `InputAction|Scope`
  (params (Key :type "Key Structure"))
  (bind _childactor (`self.ChildActor`))
  (:`Pressed`
    (if (`self.Not Reloading`)
      (`KismetSystemLibrary.MoveComponentTo` _childactor (0.0 0.0 -10.0))))
  (:`Released`
    (`KismetSystemLibrary.MoveComponentTo` _childactor (62.0 37.0 -14.0))))

(event `InputAction|Switch`
  (params (Key :type "Key Structure"))
  (:`Pressed`
    (if (`self.Not Reloading`)
      (`/Engine/EditorBlueprintResources/StandardMacros.FlipFlop`
        (:`A`
          (set `self.WhichWeapon` 0))
        (:`B`
          (set `self.WhichWeapon` 1))))))

(event `self.ReceiveBeginPlay`
  (bind _currentweapon (`self.CurrentWeapon`))
  (bind _maxammoarray (`self.MaxAmmoArray`))
  (bind (_ar _pistol _tacticalrifle) (break `/Game/Blueprints/Character/Structures/FireModeStruct` (`self.FireMode`)))
  (bind (_ar_2 _pistol_2 _tacticalrifle_2) (break `/Game/Blueprints/Character/Structures/LeftArmPosStruct` (`self.LeftArmPos`)))
  (bind (_ar_3 _pistol_3 _tacticalrifle_3) (break `/Game/Blueprints/Character/Structures/BoltPosStruct` (`self.BoltPos`)))
  (bind (_ar_4 _pistol_4 _tacticalrifle_4) (break `/Game/Blueprints/Character/Structures/ModelStruct` (`self.Model`)))
  (bind (_ar_5 _pistol_5 _tacticalrifle_5) (break `/Game/Blueprints/Character/Structures/FireRateStruct` (`self.FireRate`)))
  (bind (_ar_6 _pistol_6 _tacticalrifle_6) (break `/Game/Blueprints/Character/Structures/MagPosStruct` (`self.MagPos`)))
  (bind (_ar_7 _pistol_7 _tacticalrifle_7) (break `/Game/Blueprints/Character/Structures/ProjStruct` (`self.Projectile`)))
  (bind (_ar_8 _pistol_8 _tacticalrifle_8) (break `/Game/Blueprints/Character/Structures/ReloadTimeStruct` (`self.ReloadTime`)))
  (bind (_ar_9 _pistol_9 _tacticalrifle_9) (break `/Game/Blueprints/Character/Structures/ReloadTypeStruct` (`self.ReloadType`)))
  (bind (_ar_10 _pistol_10 _tacticalrifle_10) (break `/Game/Blueprints/Character/Structures/RightArmPosStruct` (`self.RightArmPos`)))
  (bind (_ar_11 _pistol_11 _tacticalrifle_11) (break `/Game/Blueprints/Character/Structures/MaxAmmoStruct` (`self.MaxAmmo`)))
  (set `self.speed` (`CharacterMovementComponent.MaxWalkSpeed` (`self.CharacterMovement`)))
  (set `self.FireModeArray` (`|MakeArray` _ar _pistol _tacticalrifle))
  (set `self.LeftArmPosArray` (`|MakeArray` _ar_2 _pistol_2 _tacticalrifle_2))
  (set `self.ModelArray` (`|MakeArray` _ar_4 _pistol_4 _tacticalrifle_4 :!type "Actor Class Reference"))
  (set `self.FireRateArray` (`|MakeArray` _ar_5 _pistol_5 _tacticalrifle_5))
  (set `self.MagPosArray` (`|MakeArray` _ar_6 _pistol_6 _tacticalrifle_6))
  (set `self.ProjectileArray` (`|MakeArray` _ar_7 _pistol_7 _tacticalrifle_7 :!type "Actor Class Reference"))
  (set `self.ReloadTimeArray` (`|MakeArray` _ar_8 _pistol_8 _tacticalrifle_8))
  (set `self.Reload Type Array` (`|MakeArray` _ar_9 _pistol_9 _tacticalrifle_9))
  (set `self.Right Arm Pos Array` (`|MakeArray` _ar_10 _pistol_10 _tacticalrifle_10))
  (set `self.MaxAmmoArray` (`|MakeArray` _ar_11 _pistol_11 _tacticalrifle_11))
  (set `self.BoltPosArray` (`|MakeArray` _ar_3 _pistol_3 _tacticalrifle_3))
  (set `self.PrimaryAmmo` (`|GetArrayItem` _maxammoarray (`self.Primary`)))
  (set `self.SecondaryAmmo` (`|GetArrayItem` _maxammoarray (`self.Secondary`)))
  (`KismetSystemLibrary.Delay` 0.01 :!label _label)
  (`SceneComponent.K2_SetRelativeLocation` (`self.Mag`) (`|GetArrayItem` (`self.MagPosArray`) _currentweapon) false false)
  (`SceneComponent.K2_SetRelativeLocation` (`self.Grip`) (`|GetArrayItem` (`self.LeftArmPosArray`) _currentweapon) false false)
  (`SceneComponent.K2_SetRelativeLocation` (`self.Handle`) (`|GetArrayItem` (`self.Right Arm Pos Array`) _currentweapon) false false)
  (if (`self.Not Reloading`)
    (`KismetSystemLibrary.MoveComponentTo` (`self.Cube`) (`SceneComponent.RelativeLocation` (`self.Grip`)) (struct :`Yaw` 45.0))
    (`KismetSystemLibrary.MoveComponentTo` (`self.Cube3`) (`SceneComponent.RelativeLocation` (`self.Handle`)) (struct :`Yaw` -22.5)))
  (`ChildActorComponent.SetChildActorClass` (`self.ChildActor`) (`|GetArrayItem` (`self.ModelArray`) _currentweapon))
  (`SceneComponent.K2_SetRelativeLocation` (`self.bolt`) (`|GetArrayItem` (`self.BoltPosArray`) _currentweapon) false false)
  (if (== (`self.WhichWeapon`) 0)
    (set `self.Ammo` (`KismetMathLibrary.Conv_IntToDouble` (`self.PrimaryAmmo`)))
    (set `self.CurrentWeapon` (`self.Primary`))
    (goto _label)
    (else
      (set `self.Ammo` (`KismetMathLibrary.Conv_IntToDouble` (`self.SecondaryAmmo`)))
      (set `self.CurrentWeapon` (`self.Secondary`))
      (goto _label))))

(event `InputAction|Attack`
  (params (Key :type "Key Structure"))
  (bind _firemarker (`self.FireMarker`))
  (bind _burst_counter (`self.Burst Counter`))
  (bind _returnvalue (`SceneComponent.K2_GetComponentToWorld` _firemarker))
  (bind _output (`|GetArrayItem` (`self.ProjectileArray`) (`self.CurrentWeapon`)))
  (bind _output_2 (`|GetArrayItem` (`self.FireModeArray`) (`self.CurrentWeapon`)))
  (bind _returnvalue_2 (> (`self.Ammo`) 0.0))
  (:`Pressed`
    (if _returnvalue_2
      (if (== _output_2 1)
        (if (`PlayerController.IsInputKeyDown` (`GameplayStatics.GetPlayerController` 0) Key) :!label _label_2
          (if _returnvalue_2
            (`|SpawnActorFromClass` _output _returnvalue "Undefined" "OverrideRootScale" null null)
            (`self.NewMacro_0`
              (:`Completed`
                (`self.Subract Ammo`)
                (`GameplayStatics.SpawnSoundAttached` "/Game/StarterContent/Audio/sf_laser_13.sf_laser_13" _firemarker "None" (0.0 0.0 0.0) (struct) "KeepRelativeOffset" false 1.0 1.0 0.0 null null)
                (`KismetSystemLibrary.Delay` 0.05)
                (goto _label_2)))))
        (elif (== _output_2 2)
          (`|SpawnActorFromClass` _output _returnvalue "Undefined" "OverrideRootScale" null null)
          (`self.NewMacro_0`
            (:`Completed`
              (`self.Subract Ammo`)
              (`GameplayStatics.SpawnSoundAttached` "/Game/StarterContent/Audio/laser.laser" _firemarker "None" (0.0 0.0 0.0) (struct) "KeepRelativeOffset" false 1.0 1.0 0.0 null null)))
          (else
            (set `self.Burst Counter` 0)
            (if (< _burst_counter 3) :!label _label_3
              (`|SpawnActorFromClass` (`|GetArrayItem` (`self.ProjectileArray`) (`self.CurrentWeapon`)) _returnvalue "Undefined" "OverrideRootScale" null null)
              (`self.Subract Ammo`)
              (set `self.Burst Counter` (+ _burst_counter 1))
              (`GameplayStatics.SpawnSoundAttached` "/Game/StarterContent/Audio/sf_laser_14.sf_laser_14" _firemarker "None" (0.0 0.0 0.0) (struct) "KeepRelativeOffset" false 1.0 1.0 0.0 null null)
              (`KismetSystemLibrary.Delay` 0.05)
              (goto _label_3))))))))

(fn `Subract Ammo`
  (if (== (`self.WhichWeapon`) 0)
    (set `self.PrimaryAmmo` (- (`self.PrimaryAmmo`) 1))
    (else
      (set `self.SecondaryAmmo` (- (`self.SecondaryAmmo`) 1)))))

(fn `UserConstructionScript`)