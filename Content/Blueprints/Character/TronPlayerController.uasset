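; TronPlayerController is a player controller that turns input into movement and look for player character 0.
; Look axes add yaw and inverted pitch, and move axes push the character along its actor's forward and right vectors.
; Pressing Jump starts a short-delay loop that calls Jump repeatedly while the key stays held.
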(event `InputAction|Jump`
  (params (Key :type "Key Structure"))
  (:`Pressed`
    (if (`self.IsInputKeyDown` Key) :!label _label
      (`Character.Jump` (`GameplayStatics.GetPlayerCharacter` 0))
      (`KismetSystemLibrary.Delay` 0.01)
      (goto _label))))

(event `InputAxis|LookUp`
  (params (AxisValue :type "Float (single-precision)"))
  (`Pawn.AddControllerPitchInput` (`GameplayStatics.GetPlayerCharacter` 0) (- 0.0 AxisValue)))

(event `InputAxis|LookRight`
  (params (AxisValue :type "Float (single-precision)"))
  (`Pawn.AddControllerYawInput` (`GameplayStatics.GetPlayerCharacter` 0) AxisValue))

(event `InputAxis|Left/Right`
  (params (AxisValue :type "Float (single-precision)"))
  (bind _returnvalue (`GameplayStatics.GetPlayerCharacter` 0))
  (`Pawn.AddMovementInput` _returnvalue (`KismetMathLibrary.GetRightVector` (`self.K2_GetActorRotation` _returnvalue)) AxisValue false))

(event `InputAxis|Forward/Back`
  (params (AxisValue :type "Float (single-precision)"))
  (bind _returnvalue (`GameplayStatics.GetPlayerCharacter` 0))
  (`Pawn.AddMovementInput` _returnvalue (`KismetMathLibrary.GetForwardVector` (`self.K2_GetActorRotation` _returnvalue)) AxisValue false))

(fn `UserConstructionScript`)